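; Player-controlled tank pawn Blueprint that wires input to its movement, aiming and firing.
; On BeginPlay it hands the barrel and turret meshes to TankAiming and both tracks to TankMovement.
; Move axes feed TankMovement intents, while the Fire action calls Fire.
; Aim axes rotate the camera rig, splitting yaw onto an azimuth gimbal and pitch onto the spring arm.
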(event `self.ReceiveBeginPlay`
  (`TankAimingComponent.Initialise` (`self.TankAiming`) (`self.Barrel`) (`self.Turret`))
  (`TankMovementComponent.Initialise` (`self.TankMovement`) (`self.Track_Left`) (`self.Track_Right`)))

(event `InputAxis|MoveForward`
  (params (AxisValue :type "Float (single-precision)"))
  ;[1 1 1] Movement input binding
  (`TankMovementComponent.IntendMoveForward` (`self.TankMovement`) AxisValue))

(event `InputAxis|Aim Elevation`
  (params (AxisValue :type "Float (single-precision)"))
  ;[1 1 1] Aim input binding
  (`SceneComponent.K2_AddLocalRotation` (`self.SpringArm`) (`KismetMathLibrary.MakeRotator` 0.0 AxisValue) false false))

(event `InputAxis|MoveAside`
  (params (AxisValue :type "Float (single-precision)"))
  ;[1 1 1] Movement input binding
  (`TankMovementComponent.IntendMoveAside` (`self.TankMovement`) AxisValue))

(event `InputAxis|Aim Azimuth`
  (params (AxisValue :type "Float (single-precision)"))
  ;[1 1 1] Aim input binding
  (`SceneComponent.K2_AddLocalRotation` (`self.Azimuth_Gimaball`) (`KismetMathLibrary.MakeRotator` 0.0 0.0 AxisValue) false false))

(event `InputAction|Fire`
  (params (Key :type "Key Structure"))
  ;[1 1 1] Combat actions
  (:`Pressed`
    (`self.Fire`)))

(fn `UserConstructionScript`)